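; Gameplay player controller that creates and drives the local player's UI.
; On BeginPlay, SetUpUI creates a WBP_PlayerContainer widget only for the local controller, stores it in UIRef and adds it to the viewport.
; Holding Tab shows the player list through that widget, and releasing it hides the list.
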(event `self.ReceiveBeginPlay`
  (`self.SetUpUI`))

(event `Key|Tab`
  (params (Key :type "Key Structure"))
  (:`Pressed`
    (`/Game/Torgny/UI/WBP_PlayerContainer.ShowPlayerList` (`self.UI_Ref`) true))
  (:`Released`
    (`/Game/Torgny/UI/WBP_PlayerContainer.ShowPlayerList` (`self.UI_Ref`) false)))

(fn `SetUpUI`
  (if (`self.IsLocalController`)
    (bind _returnvalue (`|CreateWidget` "/Game/Torgny/UI/WBP_PlayerContainer.WBP_PlayerContainer_C"))
    (bind _output_get (set `self.UI_Ref` _returnvalue))
    (`UserWidget.AddToViewport` _output_get 0)))

(fn `UserConstructionScript`)