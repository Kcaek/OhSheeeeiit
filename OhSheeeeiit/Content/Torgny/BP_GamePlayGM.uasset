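; Gameplay game mode that keeps a live list of connected players and shares it with every client's controller.
; PostLogin and OnLogout add or remove controllers in AllPCs, then trigger a list rebuild.
; UpdatePlayerListGM builds SPlayer entries from each PlayerState name and passes the full list to each BP_ThirdPersonPlayerController through UpdatePlayerListPC.
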(event `self.K2_PostLogin`
  (params (NewPlayer :type "PlayerController Object Reference"))
  (`KismetArrayLibrary.Array_Add` (`self.AllPCs`) NewPlayer)
  (`self.UpdatePlayerListGM` :!label _label))

(event `self.K2_OnLogout`
  (params (ExitingController :type "Controller Object Reference"))
  (bind _asplayer_controller (cast `PlayerController` ExitingController))
  (`KismetArrayLibrary.Array_RemoveItem` (`self.AllPCs`) _asplayer_controller)
  (goto _label))

(fn `UpdatePlayerListGM`
  (`KismetArrayLibrary.Array_Clear` (`self.PlayerList`))
  (for _array_element (`self.AllPCs`)
    (`KismetArrayLibrary.Array_Add` (`self.PlayerList`) (make `/Game/Torgny/S_Player` (`KismetTextLibrary.Conv_StringToText` (`PlayerState.GetPlayerName` (`Controller.PlayerState` _array_element))))))
  (for _array_element_2 (`self.AllPCs`)
    (bind _asbp_third_person_player_controller (cast `/Game/ThirdPerson/Blueprints/BP_ThirdPersonPlayerController` _array_element_2))
    (`/Game/ThirdPerson/Blueprints/BP_ThirdPersonPlayerController.UpdatePlayerListPC` _asbp_third_person_player_controller (`self.PlayerList`))))

(fn `UserConstructionScript`)