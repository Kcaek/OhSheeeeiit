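; BP_MYBLUE is a test-style trigger actor that changes the color of its Blue component when the player enters or leaves its Box.
; Box overlap events compare the other actor to player pawn 0.
; Entering prints "Ded" and applies a red material, while leaving prints "Liv" and restores blue.
; Two casts to BP_ThirdPersonCharacter are left unconnected and never run.
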(event `self.Box.OnComponentBeginOverlap`
  (params (OverlappedComponent :type "PrimitiveComponent Object Reference") (OtherActor :type "Actor Object Reference") (OtherComp :type "PrimitiveComponent Object Reference") (OtherBodyIndex :type Integer) (bFromSweep :type Boolean) (SweepResult :type "HitResult Structure (by ref)"))
  (if (== (`GameplayStatics.GetPlayerPawn` 0) OtherActor)
    (`KismetSystemLibrary.PrintString` "Ded")
    (`PrimitiveComponent.SetMaterial` (`self.Blue`) 0 "/AnimationSharing/AnimSharingRed.AnimSharingRed")))

(event `self.Box.OnComponentEndOverlap`
  (params (OverlappedComponent :type "PrimitiveComponent Object Reference") (OtherActor :type "Actor Object Reference") (OtherComp :type "PrimitiveComponent Object Reference") (OtherBodyIndex :type Integer))
  (if (== (`GameplayStatics.GetPlayerPawn` 0) OtherActor)
    (`KismetSystemLibrary.PrintString` "Liv")
    (`PrimitiveComponent.SetMaterial` (`self.Blue`) 0 "/AnimationSharing/AnimSharingBlue.AnimSharingBlue")))

(fn `UserConstructionScript`)