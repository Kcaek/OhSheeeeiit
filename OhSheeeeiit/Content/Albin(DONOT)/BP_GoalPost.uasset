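; Goal post with a moving flipbook goalkeeper that detects goals and knocks back BP_NoahTest characters.
; A timeline ping-pongs the keeper's relative location, with movement, goals and kicks routed through paired server and follow-up RPC events.
; When a ball enters the Hitbox, the last kicker scores and the goal material and keeper flipbook change during a short cooldown.
; Overlapping Fett launches the character away and briefly tilts the keeper, also behind a cooldown.
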(event `self.ReceiveBeginPlay`
  ; Moving goalkeeper
  (set `self.Relative Location` (`SceneComponent.RelativeLocation` (`self.PaperFlipbook`)))
  (`self.SPC_Server_MovePlatformToEnd`))

(event `SPC_Server_MovePlatformToEnd`
  ; Moving goalkeeper
  (`self.SPC_MovePlatformToEnd`))

(event `SPC_MovePlatformToEnd`
  ; Moving goalkeeper
  (bind (_direction _newtrack1) (`Timeline|Timeline` :!via `PlayFromStart` :!label _label)
    (:`Update`
      (`SceneComponent.K2_SetRelativeLocation` (`self.PaperFlipbook`) (+ (`self.Relative Location`) _newtrack1) false false))
    (:`Finished`
      (switch `ETimelineDirection` _direction
        (:`Forward`
          (`self.SPC_Server_MovePlatformToStart`))
        (:`Backward`
          (`self.SPC_Server_MovePlatformToEnd`))))))

(event `SPC_MovePlatformToStart`
  ; Moving goalkeeper
  (goto _label :!via `ReverseFromEnd`))

(event `SPC_Server_MovePlatformToStart`
  ; Moving goalkeeper
  (`self.SPC_MovePlatformToStart`))

(event `RPC_Server_GOAL`
  (params (FUCKYOU :type "Actor Object Reference"))
  (`self.RPC_GOAL` FUCKYOU))

(event `self.Hitbox.OnComponentBeginOverlap`
  (params (OverlappedComponent :type "PrimitiveComponent Object Reference") (OtherActor :type "Actor Object Reference") (OtherComp :type "PrimitiveComponent Object Reference") (OtherBodyIndex :type Integer) (bFromSweep :type Boolean) (SweepResult :type "HitResult Structure (by ref)"))
  (`self.RPC_Server_GOAL` OtherActor))

(event `RPC_GOAL`
  (params (FOCU :type "Actor Object Reference"))
  (bind _asbp_noah_test (cast `/Game/Noah(DoNt)/BP_NoahTest` FOCU))
  (if (`self.TempDisabled`)
    _
    (elif (== (`/Game/Noah(DoNt)/BP_NoahTest.IsBall` _asbp_noah_test) true)
      (set `self.TempDisabled` true)
      (`PrimitiveComponent.SetMaterial` (`self.MeshGoal`) 3 "/AnimationSharing/AnimSharingRed.AnimSharingRed")
      (`KismetSystemLibrary.PrintString` "GOAAAAL!!!")
      (bind _asbp_noah_test_2 (cast `/Game/Noah(DoNt)/BP_NoahTest` (`/Game/Noah(DoNt)/BP_NoahTest.LatestKick` _asbp_noah_test)))
      (bind _output_get (set `/Game/Noah(DoNt)/BP_NoahTest.CurrentScore` (+ (`/Game/Noah(DoNt)/BP_NoahTest.CurrentScore` _asbp_noah_test_2) 1) _asbp_noah_test_2))
      (`KismetSystemLibrary.PrintString` (`KismetStringLibrary.Conv_IntToString` _output_get))
      (`/Game/Noah(DoNt)/BP_NoahTest.UpdateScore` _asbp_noah_test_2)
      (`PaperFlipbookComponent.SetFlipbook` (`self.PaperFlipbook`) "/Game/EdIsDoingStuffMaybe/ShittyDoodles/FB_ed_sad_0.FB_ed_sad_0")
      (`KismetSystemLibrary.Delay` 2.0)
      (set `self.TempDisabled` false)
      (`KismetSystemLibrary.PrintString` "No longer disabled")
      (`PrimitiveComponent.SetMaterial` (`self.MeshGoal`) 3 "/Game/Tim/Material/M_Blue.M_Blue")
      (`PaperFlipbookComponent.SetFlipbook` (`self.PaperFlipbook`) "/Game/EdIsDoingStuffMaybe/ShittyDoodles/FB_ed_distressed_0.FB_ed_distressed_0"))))

(event `RPC_Server_KickGoal`
  (`self.RPC_KickGoal`))

(event `self.fett.OnComponentBeginOverlap`
  (params (OverlappedComponent :type "PrimitiveComponent Object Reference") (OtherActor :type "Actor Object Reference") (OtherComp :type "PrimitiveComponent Object Reference") (OtherBodyIndex :type Integer) (bFromSweep :type Boolean) (SweepResult :type "HitResult Structure (by ref)"))
  (bind _asbp_noah_test (cast `/Game/Noah(DoNt)/BP_NoahTest` OtherActor))
  (`KismetSystemLibrary.PrintString` "Nonono")
  (if (not (`self.TempKickDisabled`))
    (`self.RPC_Server_KickGoal`)))

(event `RPC_KickGoal`
  (set `self.TempKickDisabled` true)
  (`Character.LaunchCharacter` (stale `self.fett.OnComponentBeginOverlap` _asbp_noah_test) (-5000.0 0.0 0.0) false false)
  (`SceneComponent.K2_AddRelativeRotation` (`self.PaperFlipbook`) (`KismetMathLibrary.MakeRotator` -20.0) false false)
  (`KismetSystemLibrary.Delay` 1.0)
  (`SceneComponent.K2_AddRelativeRotation` (`self.PaperFlipbook`) (`KismetMathLibrary.MakeRotator` 20.0) false false)
  (set `self.TempKickDisabled` false))

(fn `UserConstructionScript`)